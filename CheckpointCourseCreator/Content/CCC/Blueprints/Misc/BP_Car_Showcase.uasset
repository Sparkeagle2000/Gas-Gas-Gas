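; BP_Car_Showcase is a showcase car actor with left and right doors that can be toggled open and closed.
; Each door event flips an open flag and plays or reverses its own timeline, which writes the door's open value to a variable.
; The construction script adds a static mesh CCC badge and snaps it to the SteeringWheelBadge socket on the Car component.
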(event `LeftDoor`
  ;[0 0 0] Left Door interaction
  (if (`self.LeftDoorOpen`)
    (set `self.LeftDoorOpen` false)
    (bind (_direction _leftdooropenvalue) (`Timeline|LeftDoorTimeline` :!via `Reverse` :!label _label)
      (:`Update`
        (set `self.LeftDoorOpenValue` _leftdooropenvalue)))
    (else
      (set `self.LeftDoorOpen` true)
      (goto _label))))

(event `RightDoor`
  ;[0 0 0] Right Door interaction
  (if (`self.RightDoorOpen`)
    (set `self.RightDoorOpen` false)
    (bind (_direction _rightdooropenvalue) (`Timeline|RightDoorTimeline` :!via `Reverse` :!label _label_2)
      (:`Update`
        (set `self.RightDoorOpenValue` _rightdooropenvalue)))
    (else
      (set `self.RightDoorOpen` true)
      (goto _label_2))))

(fn `UserConstructionScript`
  ;[0 0 0] Attach CCC badge to steering wheel
  ;;[1 1 1] Create CCC badge for Steering Wheel
  (bind _returnvalue (`AddComponent|NODE_AddStaticMeshComponent-0` :`bManualAttachment` true))
  ;;[1 1 1] Attach badges
  (`SceneComponent.K2_AttachToComponent` _returnvalue (`self.Car`) "SteeringWheelBadge" "SnapToTarget" "SnapToTarget" "SnapToTarget" false))