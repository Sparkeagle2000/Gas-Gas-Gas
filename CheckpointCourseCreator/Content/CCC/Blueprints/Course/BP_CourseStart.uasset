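; BP_CourseStart is a race course start marker that offers BP_Car a race start prompt.
; While Active, its sphere overlap sets the car's prompt flag and a reference to this start, then clears both on exit.
; Overlaps accept vehicles or characters, but the cast means only BP_Car responds.
; An Activate/Deactivate event shows or hides the static mesh to match Active.
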(event `Activate/Deactivate`
  ;[0 0 0] Activate/Deactivate events
  (if (`self.Active`)
    (`SceneComponent.SetHiddenInGame` (`self.StaticMesh`) false false)
    (else
      (`SceneComponent.SetHiddenInGame` (`self.StaticMesh`) true false))))

(event `self.Sphere.OnComponentBeginOverlap`
  (params (OverlappedComponent :type "PrimitiveComponent Object Reference") (OtherActor :type "Actor Object Reference") (OtherComp :type "PrimitiveComponent Object Reference") (OtherBodyIndex :type Integer) (bFromSweep :type Boolean) (SweepResult :type "HitResult Structure (by ref)"))
  (bind _returnvalue (`GameplayStatics.GetObjectClass` OtherActor))
  ;[0 0 0] Overlap events
  ;;[1 1 1] If overlapping actor = vehicle or character
  (if (and (or (`KismetMathLibrary.ClassIsChildOf` _returnvalue "/Script/PhysXVehicles.WheeledVehicle") (`KismetMathLibrary.ClassIsChildOf` _returnvalue "/Script/Engine.Character")) (`self.Active`))
    ;;[1 1 1] Set race start prompt and start reference in Car blueprint
    (bind _asbp_car (cast `/Game/CCC/Blueprints/BP_Car` OtherActor))
    (bind _output_get (set `self.CarBPReference` _asbp_car))
    (set `/Game/CCC/Blueprints/BP_Car.RaceStartPrompt` true _output_get)
    (set `/Game/CCC/Blueprints/BP_Car.RaceStartReference` self _output_get)))

(event `self.Sphere.OnComponentEndOverlap`
  (params (OverlappedComponent :type "PrimitiveComponent Object Reference") (OtherActor :type "Actor Object Reference") (OtherComp :type "PrimitiveComponent Object Reference") (OtherBodyIndex :type Integer))
  (bind _returnvalue (`GameplayStatics.GetObjectClass` OtherActor))
  ;[0 0 0] Overlap events
  ;;[1 1 1] If overlapping actor = vehicle or character
  (if (and (or (`KismetMathLibrary.ClassIsChildOf` _returnvalue "/Script/PhysXVehicles.WheeledVehicle") (`KismetMathLibrary.ClassIsChildOf` _returnvalue "/Script/Engine.Character")) (`self.Active`))
    ;;[1 1 1] Set race start prompt and start reference in Car blueprint
    (bind _asbp_car (cast `/Game/CCC/Blueprints/BP_Car` OtherActor))
    (bind _output_get (set `self.CarBPReference` _asbp_car))
    (set `/Game/CCC/Blueprints/BP_Car.RaceStartPrompt` false _output_get)
    (set `/Game/CCC/Blueprints/BP_Car.RaceStartReference` null _output_get)))

(fn `UserConstructionScript`)