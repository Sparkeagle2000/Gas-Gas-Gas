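; Checkpoint actor for a race course, colored by active, inactive or finish state, with grounded (capsule) and flying (sphere) variants.
; When a vehicle or character overlaps it, it advances the course blueprint's counters and activates the next checkpoint or lap.
; The last one ends the course, spawns a finish camera, then re-enables course starts and destroys all checkpoints.
; Construction applies meshes, visibility and final-point behavior, optionally aligning the finish point with the previous one.
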(event `Finish`
  (bind _coursebpreference (`self.CourseBPReference`))
  (bind _carbpreference (`self.CarBPReference`))
  ;[0 0 0] Finish events
  ;;[0 0 0] Deactivate self
  (`self.Activate/Deactivate` false false true)
  ;;[1 1 1] Set course as inactive and set off Finish events in course BP
  (set `/Game/CCC/Blueprints/Course/BP_Course.CourseActive` false _coursebpreference)
  (`/Game/CCC/Blueprints/Course/BP_Course.Finish` _coursebpreference)
  (`|ExecutionSequence`
    (:`then_0`
      ;;[1 1 1] Spawn camera crane and set variables in that blueprint
      (bind _asbp_car (cast `/Game/CCC/Blueprints/BP_Car` (`self.PlayerActor`)))
      (bind _output_get (set `self.CarBPReference` _asbp_car))
      (`/Game/CCC/Blueprints/Widgets/W_CarWidget.PlayBlurAnimation` (`/Game/CCC/Blueprints/BP_Car.CarWidget` _output_get))
      (`|SpawnActorFromClass` (`/Game/CCC/Blueprints/Course/BP_Course.FinishCameraClass` (`self.CourseBPReference`)) (`KismetMathLibrary.MakeTransform` (`self.K2_GetActorLocation`)) "Undefined" "OverrideRootScale" null _asbp_car self null))
    (:`then_1`
      _))
  ;;[1 1 1] Delay
  (`KismetSystemLibrary.Delay` (+ (`/Game/CCC/Blueprints/Course/BP_Course.FinishCamDuration` (`self.CourseBPReference`)) 0.1))
  ;;[1 1 1] Set current time to 0
  (set `/Game/CCC/Blueprints/Course/BP_Course.CurrentTime` 0.0 (`self.CourseBPReference`))
  ;;[1 1 1] Set not participating in course and disable finish screen visibility (Hides course info in Widget)
  (set `/Game/CCC/Blueprints/BP_Car.ParticipatingInCourse` false _carbpreference)
  (set `/Game/CCC/Blueprints/Widgets/W_CarWidget.FinishScreenVisibility` false (`/Game/CCC/Blueprints/BP_Car.CarWidget` _carbpreference))
  ;;[1 1 1] Reactivate race start blueprints
  (bind _outactors (`GameplayStatics.GetAllActorsOfClass` "/Game/CCC/Blueprints/Course/BP_CourseStart.BP_CourseStart_C"))
  (for _array_element _outactors
    (set `/Game/CCC/Blueprints/Course/BP_CourseStart.Active` true _array_element)
    (`/Game/CCC/Blueprints/Course/BP_CourseStart.Activate/Deactivate` _array_element))
  ;;[1 1 1] Destroy all checkpoints
  (for _array_element_2 (`/Game/CCC/Blueprints/Course/BP_Course.CheckpointActors` (`self.CourseBPReference`))
    (`self.K2_DestroyActor` _array_element_2)))

(event `self.Sphere.OnComponentBeginOverlap`
  (params (OverlappedComponent :type "PrimitiveComponent Object Reference") (OtherActor :type "Actor Object Reference") (OtherComp :type "PrimitiveComponent Object Reference") (OtherBodyIndex :type Integer) (bFromSweep :type Boolean) (SweepResult :type "HitResult Structure (by ref)"))
  (bind _coursebpreference (`self.CourseBPReference`))
  (bind _coursebpreference_2 (`self.CourseBPReference`))
  (bind _coursebpreference_3 (`self.CourseBPReference`))
  (bind _coursebpreference_4 (`self.CourseBPReference`))
  (bind _coursebpreference_5 (`self.CourseBPReference`))
  (bind _coursebpreference_6 (`self.CourseBPReference`))
  ;[0 0 0] If overlapping actor = vehicle or character
  (bind _output_get (set `self.PlayerActor` OtherActor))
  (bind _returnvalue (`GameplayStatics.GetObjectClass` _output_get))
  (bind _returnvalue_2 (`GameplayStatics.GetObjectClass` (stale `self.Capsule.OnComponentBeginOverlap` _output_get)))
  (if (or (`KismetMathLibrary.ClassIsChildOf` _returnvalue "/Script/PhysXVehicles.WheeledVehicle") (`KismetMathLibrary.ClassIsChildOf` _returnvalue "/Script/Engine.Character") (`KismetMathLibrary.ClassIsChildOf` _returnvalue_2 "/Script/PhysXVehicles.WheeledVehicle") (`KismetMathLibrary.ClassIsChildOf` _returnvalue_2 "/Script/Engine.Character")) :!label _label
    ;[0 0 0] Set self as inactive
    (`self.Activate/Deactivate` false)
    ;[0 0 0] Set next checkpoint index
    (`self.NextCheckpointMath`)
    (`self.CheckIfFinalCheckpoint`
      (:`Finish Checkpoint`
        ;[0 0 0] Finish event
        (`self.Finish`))
      (:`Not Finish`
        ;[0 0 0] If overlapped last checkpoint in lap
        (if (== (`/Game/CCC/Blueprints/Course/BP_Course.CurrentLapCheckpoint` _coursebpreference_4) (`KismetArrayLibrary.Array_Length` (`/Game/CCC/Blueprints/Course/BP_Course.Checkpoints` _coursebpreference_4)))
          ;[0 0 0] Lap events
          ;;[1 1 1] If there is only one checkpoint, finish course regardless of lap count
          (if (> (`KismetArrayLibrary.Array_Length` (`/Game/CCC/Blueprints/Course/BP_Course.Checkpoints` (`self.CourseBPReference`))) 1)
            ;;[1 1 1] Increase lap count
            (set `/Game/CCC/Blueprints/Course/BP_Course.CurrentCourseLap` (`KismetMathLibrary.Clamp` (+ (`/Game/CCC/Blueprints/Course/BP_Course.CurrentCourseLap` _coursebpreference) 1) 1 (`/Game/CCC/Blueprints/Course/BP_Course.Laps` _coursebpreference)) (`self.CourseBPReference`))
            ;;[1 1 1] Loop lap checkpoint index
            (set `/Game/CCC/Blueprints/Course/BP_Course.CurrentLapCheckpoint` 0 (`self.CourseBPReference`))
            ;;[1 1 1] Activate first checkpoint to start next lap
            (`self.Activate/Deactivate` (`|GetArrayItem` (`/Game/CCC/Blueprints/Course/BP_Course.CheckpointActors` _coursebpreference_5) (`/Game/CCC/Blueprints/Course/BP_Course.CurrentLapCheckpoint` _coursebpreference_5)) true false true)
            ;;[1 1 1] If final lap, execute finish point behavior
            (if (== (`/Game/CCC/Blueprints/Course/BP_Course.CurrentCourseLap` _coursebpreference_3) (`/Game/CCC/Blueprints/Course/BP_Course.Laps` _coursebpreference_3))
              (`self.FinalPointBehaviorFunction` false))
            (else
              (`self.Finish`)
              (`KismetSystemLibrary.PrintString` "Course cannot lap as there is only one checkpoint" true true (struct :`R` 1.0 :`A` 1.0) 10.0)))
          (else
            ;[0 0 0] Activate next checkpoint
            (`self.Activate/Deactivate` (`|GetArrayItem` (`/Game/CCC/Blueprints/Course/BP_Course.CheckpointActors` _coursebpreference_6) (`/Game/CCC/Blueprints/Course/BP_Course.CurrentLapCheckpoint` _coursebpreference_6)) true (== (`/Game/CCC/Blueprints/Course/BP_Course.CurrentCourseCheckpoint` _coursebpreference_2) (- (`/Game/CCC/Blueprints/Course/BP_Course.CourseTotalCheckpoints` _coursebpreference_2) 1)) true)))))))

(event `self.Capsule.OnComponentBeginOverlap`
  (params (OverlappedComponent :type "PrimitiveComponent Object Reference") (OtherActor :type "Actor Object Reference") (OtherComp :type "PrimitiveComponent Object Reference") (OtherBodyIndex :type Integer) (bFromSweep :type Boolean) (SweepResult :type "HitResult Structure (by ref)"))
  ;[0 0 0] If overlapping actor = vehicle or character
  (bind _output_get (set `self.PlayerActor` OtherActor))
  (goto _label))

(fn `Activate/Deactivate`
  (params (`Activate/Deactivate` :type Boolean) (ColorAsFinalCheckpoint :type Boolean) (PlaySound :type Boolean))
  (if `Activate/Deactivate`
    ;[0 0 0] Activate
    (set `self.Active` true)
    (`SceneComponent.SetVisibility` (`self.Marker`) true true)
    (`SceneComponent.SetVisibility` (`self.Point`) true true)
    (`SceneComponent.SetVisibility` (`self.ParticleSystem`) true true)
    (`self.SetCollisionShape`)
    (`self.SetColor` (select `bool` ColorAsFinalCheckpoint :`false` (`self.ActiveColor`) :`true` (`self.FinishColor`)))
    (`LightComponent.SetLightColor` (`self.PointLight`) (select `bool` ColorAsFinalCheckpoint :`false` (`self.ActiveColor`) :`true` (`self.FinishColor`)) true)
    ;;[1 1 1] If final checkpoint, and Finish Point Behavior = Hide Point
    (if (and ColorAsFinalCheckpoint (`|EnumEquality` (`self.FinalPointBehavior`) "NewEnumerator0"))
      ;;[1 1 1] Hide point
      (`SceneComponent.SetVisibility` (`self.Point`) false false))
    (else
      ;[0 0 0] Deactivate
      (set `self.Active` false)
      (set `PrimitiveComponent.bGenerateOverlapEvents` false (`self.Sphere`))
      (set `PrimitiveComponent.bGenerateOverlapEvents` false (`self.Capsule`))
      (`self.SetColor` (`self.InactiveColor`))
      (`LightComponent.SetLightColor` (`self.PointLight`) (`self.InactiveColor`) true)
      ;;[1 1 1] Hide mesh components if Visibility set to Only Active Checkpoint
      (if (select `/Game/CCC/Blueprints/Enums/E_CheckpointVisibility` (`self.Visibility`) :`NewEnumerator0` true)
        (`SceneComponent.SetVisibility` (`self.Marker`) false false)
        (`SceneComponent.SetVisibility` (`self.Point`) false false)
        (`SceneComponent.SetVisibility` (`self.ParticleSystem`) false false))))
  ;[0 0 0] Play sound
  (if PlaySound
    (`GameplayStatics.PlaySound2D` (`self.ActivateSound`) 1.0 1.0 0.0 null null)))

(fn `FinalPointBehaviorFunction`
  (params (OnConstruct :type Boolean))
  (locals (`OnConstruct/OnLap` :type Boolean) (FinishBehaviorPoint :type "StaticMeshComponent Object Reference"))
  (bind _checkpointactors (`/Game/CCC/Blueprints/Course/BP_Course.CheckpointActors` (`self.CourseBPReference`)))
  (bind _checkpointactors_2 (`/Game/CCC/Blueprints/Course/BP_Course.CheckpointActors` (`self.CourseBPReference`)))
  ;[0 0 0] Set Final Point Behavior
  (bind _output_get (set `local.OnConstruct/OnLap` OnConstruct)) ; If on construct or lap event
  ;;[1 1 1] If on construct, set events for local point. If on lap = set events for finish point
  (set `local.FinishBehaviorPoint` (select `bool` _output_get :`false` (`/Game/CCC/Blueprints/Course/Checkpoints/BP_Checkpoint.Point` (`|GetArrayItem` _checkpointactors (- (`KismetArrayLibrary.Array_Length` _checkpointactors) 1))) :`true` (`self.Point`)))
  ;;[1 1 1] Select based on Finish Point Behavior
  (`|MultiGate` false false (select `/Game/CCC/Blueprints/Enums/E_FinalPointBehavior` (`self.FinalPointBehavior`) :`NewEnumerator1` 1 :`NewEnumerator2` 2)
    (:`Out 0`
      ;;[1 1 1] Hide point
      (`SceneComponent.SetVisibility` (`local.FinishBehaviorPoint`) false false))
    (:`Out 1`
      ;;[1 1 1] Only continue if there is more than one checkpoint, or there won't be a previous point to reference
      (if (> (`KismetArrayLibrary.Array_Length` (`/Game/CCC/Blueprints/Course/BP_Course.CheckpointActors` (`self.CourseBPReference`))) 1)
        ;;[1 1 1] Set rotation of finish point
        (`SceneComponent.K2_SetWorldRotation` (`local.FinishBehaviorPoint`) (`KismetMathLibrary.FindLookAtRotation` (`SceneComponent.K2_GetComponentLocation` (`/Game/CCC/Blueprints/Course/Checkpoints/BP_Checkpoint.Point` (`|GetArrayItem` _checkpointactors_2 (- (`KismetArrayLibrary.Array_Length` _checkpointactors_2) (select `bool` (`local.OnConstruct/OnLap`) :`false` 2 :`true` 1))))) (`SceneComponent.K2_GetComponentLocation` (`local.FinishBehaviorPoint`))) false false)))))

(fn `NextCheckpointMath`
  (bind _coursebpreference (`self.CourseBPReference`))
  ;[0 0 0] Set next checkpoint increment for lap and course
  ;;[1 1 1] Current course checkpoint
  (set `/Game/CCC/Blueprints/Course/BP_Course.CurrentCourseCheckpoint` (`KismetMathLibrary.Clamp` (+ (`/Game/CCC/Blueprints/Course/BP_Course.CurrentCourseCheckpoint` _coursebpreference) 1) 0 (`/Game/CCC/Blueprints/Course/BP_Course.CourseTotalCheckpoints` _coursebpreference)) (`self.CourseBPReference`))
  ;;[1 1 1] Current Lap checkpoint
  (set `/Game/CCC/Blueprints/Course/BP_Course.CurrentLapCheckpoint` (+ (`/Game/CCC/Blueprints/Course/BP_Course.CurrentLapCheckpoint` (`self.CourseBPReference`)) 1) (`self.CourseBPReference`)))

(fn `SetCollisionShape`
  ;[0 0 0] Set overlap collision shape for checkpoint type, grounded will use a capsule while air will use a sphere
  (if (select `/Game/CCC/Blueprints/Enums/E_CheckpointType_PerIndex` (`self.CT`) :`NewEnumerator1` true)
    (set `PrimitiveComponent.bGenerateOverlapEvents` true (`self.Capsule`))
    (set `PrimitiveComponent.bGenerateOverlapEvents` false (`self.Sphere`))
    (else
      (set `PrimitiveComponent.bGenerateOverlapEvents` false (`self.Capsule`))
      (set `PrimitiveComponent.bGenerateOverlapEvents` true (`self.Sphere`)))))

(fn `SetColor`
  (params (Color :type "LinearColor Structure"))
  ;[0 0 0] Set color
  (`|ExecutionSequence`
    (:`then_0`
      (if (and (`self.ColorPoint`) (> (`PrimitiveComponent.GetNumMaterials` (`self.Point`)) 0))
        (bind _returnvalue (`PrimitiveComponent.CreateDynamicMaterialInstance` (`self.Point`) 0 null "None"))
        (`/Engine/EditorBlueprintResources/StandardMacros.IsValid` _returnvalue
          (:`Is Valid`
            (`MaterialInstanceDynamic.SetVectorParameterValue` _returnvalue "Color" Color)))))
    (:`then_1`
      (if (and (`self.ColorMarker`) (> (`PrimitiveComponent.GetNumMaterials` (`self.Marker`)) 0))
        (bind _returnvalue_2 (`PrimitiveComponent.CreateDynamicMaterialInstance` (`self.Marker`) 0 null "None"))
        (`/Engine/EditorBlueprintResources/StandardMacros.IsValid` _returnvalue_2
          (:`Is Valid`
            (`MaterialInstanceDynamic.SetVectorParameterValue` _returnvalue_2 "Color" Color)))))
    (:`then_2`
      (if (`self.ColorParticle`)
        (`ParticleSystemComponent.SetColorParameter` (`self.ParticleSystem`) "Color" Color)))))

(fn `UserConstructionScript`
  (bind _coursebpreference (`self.CourseBPReference`))
  (bind _coursebpreference_2 (`self.CourseBPReference`))
  (`/Engine/EditorBlueprintResources/StandardMacros.IsValid` (`self.CourseBPReference`)
    (:`Is Valid`
      (`|ExecutionSequence`
        (:`then_0`
          ;[0 0 0] Construct point, marker and particle
          ;;[1 1 1] Set point and marker rotations
          (`SceneComponent.K2_SetWorldRotation` (`self.Marker`) (`self.MarkerRotation`) false false)
          (`SceneComponent.K2_SetWorldRotation` (`self.Point`) (`self.PointRotation`) false false)
          ;;[1 1 1] Set Particle System if valid
          (`/Engine/EditorBlueprintResources/StandardMacros.IsValid` (`self.ParticleSystem`)
            (:`Is Valid`
              (`ParticleSystemComponent.SetTemplate` (`self.ParticleSystem`) (`self.Particle`))
              ;;[1 1 1] Set Point Mesh if valid
              (`/Engine/EditorBlueprintResources/StandardMacros.IsValid` (`self.Point`)
                (:`Is Valid`
                  (`StaticMeshComponent.SetStaticMesh` (`self.Point`) (`self.PointMesh`)))
                (:`Is Not Valid`
                  _))
              ;;[1 1 1] Set marker mesh based on checkpoint type
              (`/Engine/EditorBlueprintResources/StandardMacros.IsValid` (`StaticMeshComponent.StaticMesh` (`self.Marker`))
                (:`Is Valid`
                  (`StaticMeshComponent.SetStaticMesh` (`self.Marker`) (select `/Game/CCC/Blueprints/Enums/E_CheckpointType_PerIndex` (`self.CT`) :`NewEnumerator1` (`self.GroundedMarkerMesh`) :`NewEnumerator0` (`self.FlyingMarkerMesh`))))
                (:`Is Not Valid`
                  _))
              ;;[1 1 1] Set inactive color
              (`self.SetColor` (`self.InactiveColor`))
              ;;[1 1 1] Set Light Color
              (`LightComponent.SetLightColor` (`self.PointLight`) (`self.InactiveColor`) true)
              ;;[1 1 1] Add offset for arrow if grounded checkpoint type
              (if (select `/Game/CCC/Blueprints/Enums/E_CheckpointType_PerIndex` (`self.CT`) :`NewEnumerator1` true)
                (`SceneComponent.K2_AddWorldOffset` (`self.Point`) (`KismetMathLibrary.MakeVector` 0.0 0.0 (`self.ArrowZOffset`)) false false)))))
        (:`then_1`
          ;[0 0 0] Hide mesh components if visibility set to only active
          (if (select `/Game/CCC/Blueprints/Enums/E_CheckpointVisibility` (`self.Visibility`) :`NewEnumerator0` true)
            ;;[1 1 1] If first checkpoint, do not hide
            (if (not (== (`self.CheckpointIndex`) 0))
              (`SceneComponent.SetVisibility` (`self.Marker`) false false)
              (`SceneComponent.SetVisibility` (`self.Point`) false false)
              (`SceneComponent.SetVisibility` (`self.ParticleSystem`) false false))))
        (:`then_2`
          ;[0 0 0] Set finish checkpoint behavior If only one lap, and is last checkpoint
          (if (and (not (> (`/Game/CCC/Blueprints/Course/BP_Course.Laps` _coursebpreference) 1)) (== (`self.CheckpointIndex`) (- (`KismetArrayLibrary.Array_Length` (`/Game/CCC/Blueprints/Course/BP_Course.Checkpoints` _coursebpreference)) 1)))
            (`self.FinalPointBehaviorFunction` true)))
        (:`then_3`
          ;[0 0 0] Set active if current active checkpoint
          (if (== (`self.CheckpointIndex`) (`/Game/CCC/Blueprints/Course/BP_Course.CurrentLapCheckpoint` _coursebpreference_2))
            (set `self.Active` true)
            (else
              (set `self.Active` false)))
          (`self.Activate/Deactivate` (`self.Active`) (and (not (> (`KismetArrayLibrary.Array_Length` (`/Game/CCC/Blueprints/Course/BP_Course.Checkpoints` _coursebpreference_2)) 1)) (not (> (`/Game/CCC/Blueprints/Course/BP_Course.Laps` _coursebpreference_2) 1)))))))))