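; Finish line crane camera that temporarily takes over the player's view and tracks their car.
; Construction offsets it from the checkpoint and sets the starting crane values.
; After a brief delay it becomes the view target, then returns the view to the car after the course's finish-cam duration and destroys itself.
; Each tick eases crane pitch, yaw and arm length toward targets and aims the camera at the car.
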(event `self.ReceiveBeginPlay`
  ;[0 0 0] Switch camera event
  (`KismetSystemLibrary.Delay` 0.1) ; Allows a frame to set camera rotation
  (bind _asplayer_controller (cast `PlayerController` (`Pawn.GetController` (`self.PlayerCarReference`))))
  (bind _output_get (set `self.PlayerController` _asplayer_controller))
  (`PlayerController.SetViewTargetWithBlend` _output_get self 0.0 "VTBlend_Linear" 0.0 false)
  (`KismetSystemLibrary.Delay` (`/Game/CCC/Blueprints/Course/BP_Course.FinishCamDuration` (`/Game/CCC/Blueprints/Course/Checkpoints/BP_Checkpoint.CourseBPReference` (`self.FinishCheckpoint`))))
  (`PlayerController.SetViewTargetWithBlend` (`self.PlayerController`) (`self.PlayerCarReference`) 0.0 "VTBlend_Linear" 0.0 false)
  (`self.K2_DestroyActor`))

(event `self.ReceiveTick`
  (params (DeltaSeconds :type "Float (single-precision)"))
  ;[0 0 0] Camera crane movement
  (`/Engine/EditorBlueprintResources/StandardMacros.IsValid` (`self.PlayerCarReference`)
    (:`Is Valid`
      (set `self.CranePitch` (`KismetMathLibrary.FInterpTo` (`self.CranePitch`) (`self.Pitch_Target`) (`GameplayStatics.GetWorldDeltaSeconds`) 0.1))
      (set `self.CraneYaw` (`KismetMathLibrary.FInterpTo` (`self.CraneYaw`) (`self.Yaw_Target`) (`GameplayStatics.GetWorldDeltaSeconds`) 0.1))
      (set `self.CraneArmLength` (`KismetMathLibrary.FInterpTo` (`self.CraneArmLength`) (`self.ArmlLength_Target`) (`GameplayStatics.GetWorldDeltaSeconds`) (`self.ArmLength_Speed`)))
      (`SceneComponent.K2_SetWorldRotation` (`self.Camera`) (`KismetMathLibrary.FindLookAtRotation` (`SceneComponent.K2_GetComponentLocation` (`self.Camera`)) (`self.K2_GetActorLocation` (`self.PlayerCarReference`))) false false))))

(fn `UserConstructionScript`
  ;[0 0 0] Camera crane construction
  ;;[1 1 1] Add offset from checkpoint
  (`self.K2_AddActorLocalOffset` (`self.OffsetFromCheckpoint`))
  ;;[1 1 1] Set start crane settings
  (set `self.CranePitch` (`self.Pitch_Start`))
  (set `self.CraneYaw` (`self.Yaw_Start`))
  (set `self.CraneArmLength` (`self.ArmlLength_Target`)))